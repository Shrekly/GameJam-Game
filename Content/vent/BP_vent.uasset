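; BP_vent is an interactable vent the player opens by unscrewing its four screws with a mouse cursor.
; Interacting, if the character's screwdriver check passes, freezes movement and look and blends the view to the vent.
; Each screw's click plays a one-shot timeline sliding it out, then enables physics and increments ScrewCount.
; Once all four are out, player control and camera are restored and a timeline rotates the cover open.
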(event OnClicked(vent2_Circle_005)
  (params (TouchedComponent :type Primitive%20Component%20Object%20Reference) (ButtonPressed :type Key%20Structure :default "None"))
  (Development|PrintString (Utilities|GetDisplayName TouchedComponent))
  (Utilities|FlowControl|DoOnce false
    (:Completed
      (bind _newtrack_0 (Timeline|Timeline Play)
        (:Update
          (Transformation|SetRelativeLocation TouchedComponent (Math|Vector|MakeVector 0.0 (Math|Float|Lerp 0.0 4.0 _newtrack_0) 0.0) false false))
        (:Finished
          (Physics|SetSimulatePhysics TouchedComponent true)
          (bind _result (Math|Integer|IncrementInt (Variables|Default|Getscrew%20count))
            (:%20%20
              (Variables|Default|Setscrew%20count _result)
              (CallFunction|OpenVent))))))))

(event OnClicked(vent2_Circle_002)
  (params (TouchedComponent :type Primitive%20Component%20Object%20Reference) (ButtonPressed :type Key%20Structure :default "None"))
  (Development|PrintString (Utilities|GetDisplayName TouchedComponent))
  (Utilities|FlowControl|DoOnce false
    (:Completed
      (bind _newtrack_0 (Timeline|Timeline_0 Play)
        (:Update
          (Transformation|SetRelativeLocation TouchedComponent (Math|Vector|MakeVector 0.0 (Math|Float|Lerp 0.0 4.0 _newtrack_0) 0.0) false false))
        (:Finished
          (Physics|SetSimulatePhysics TouchedComponent true)
          (bind _result (Math|Integer|IncrementInt (Variables|Default|Getscrew%20count))
            (:%20%20
              (Variables|Default|Setscrew%20count _result)
              (CallFunction|OpenVent))))))))

(event OnClicked(vent2_Circle_007)
  (params (TouchedComponent :type Primitive%20Component%20Object%20Reference) (ButtonPressed :type Key%20Structure :default "None"))
  (Development|PrintString (Utilities|GetDisplayName TouchedComponent))
  (Utilities|FlowControl|DoOnce false
    (:Completed
      (bind _newtrack_0 (Timeline|Timeline_1 Play)
        (:Update
          (Transformation|SetRelativeLocation TouchedComponent (Math|Vector|MakeVector 0.0 (Math|Float|Lerp 0.0 4.0 _newtrack_0) 0.0) false false))
        (:Finished
          (Physics|SetSimulatePhysics TouchedComponent true)
          (bind _result (Math|Integer|IncrementInt (Variables|Default|Getscrew%20count))
            (:%20%20
              (Variables|Default|Setscrew%20count _result)
              (CallFunction|OpenVent))))))))

(event OnClicked(vent2_Circle_004)
  (params (TouchedComponent :type Primitive%20Component%20Object%20Reference) (ButtonPressed :type Key%20Structure :default "None"))
  (Development|PrintString (Utilities|GetDisplayName TouchedComponent))
  (Utilities|FlowControl|DoOnce false
    (:Completed
      (bind _newtrack_0 (Timeline|Timeline_2 Play)
        (:Update
          (Transformation|SetRelativeLocation TouchedComponent (Math|Vector|MakeVector 0.0 (Math|Float|Lerp 0.0 4.0 _newtrack_0) 0.0) false false))
        (:Finished
          (Physics|SetSimulatePhysics TouchedComponent true)
          (bind _result (Math|Integer|IncrementInt (Variables|Default|Getscrew%20count))
            (:%20%20
              (Variables|Default|Setscrew%20count _result)
              (CallFunction|OpenVent))))))))

(event Custom|open%20vent
  (bind _returnvalue (Game|GetPlayerController 0))
  (if (>= (Variables|Default|Getscrew%20count) 4)
    (Pawn|Components|CharacterMovement|SetMovementMode (Variables|/Script/Engine.Character|GetCharacterMovement (Game|GetPlayerCharacter 0)) "MOVE_Walking" 0)
    (Input|ResetIgnoreLookInput _returnvalue)
    (Variables|/Script/Engine.PlayerController|SetbEnableClickEvents _returnvalue false)
    (Variables|/Script/Engine.PlayerController|SetbShowMouseCursor _returnvalue false)
    (Game|Player|SetViewTargetwithBlend _returnvalue (Game|GetPlayerCharacter 0) 0.3 "VTBlend_Linear" 0.0 false)
    (Input|SetInputModeGameOnly _returnvalue false)
    (bind _newtrack_0 (Timeline|Timeline_3 Play)
      (:Update
        (Transformation|SetRelativeRotation (Variables|Default|Getvent2_Cube) (Math|Rotator|MakeRotator (Math|Float|Lerp 0.0 9e+01 _newtrack_0) 0.0 0.0) false false)))))

(event EventInteract
  (bind _returnvalue (Game|GetPlayerController 0))
  (bind _has_screw_driver (Class|BPIScrewdriver|SetScrewDriver(Message) (Game|GetPlayerCharacter 0)))
  (if _has_screw_driver
    (Pawn|Components|CharacterMovement|DisableMovement (Variables|/Script/Engine.Character|GetCharacterMovement (Game|GetPlayerCharacter 0)))
    (Input|SetIgnoreLookInput _returnvalue true)
    (Input|EnableInput _returnvalue)
    (Variables|/Script/Engine.PlayerController|SetbEnableClickEvents _returnvalue true)
    (Variables|/Script/Engine.PlayerController|SetbShowMouseCursor _returnvalue true)
    (Game|Player|SetViewTargetwithBlend _returnvalue self 0.4 "VTBlend_Linear" 0.0 false)))

(fn ConstructionScript)