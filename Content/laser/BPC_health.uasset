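; BPC_health is a Blueprint component that stores a Health value and exposes functions to raise or lower it.
; IncreaseHealth adds an amount and clamps the result between zero and one hundred.
; Decreasehealth subtracts damage without clamping, then reaches an empty branch, while a check for zero or lower health sits unconnected.
; The event graph is empty apart from disabled BeginPlay and Tick stubs.
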(event EventBeginPlay)

(event EventTick
  (params (DeltaSeconds :type Float%20%28single-precision%29)))

(fn IncreaseHealth
  (params (amount :type Float%20%28double-precision%29))
  (Variables|Default|Sethealth (Math|Float|Clamp(Float) (+ (Variables|Default|Gethealth) amount) 0.0 1e+02)))

(fn Decreasehealth
  (params (damage :type Float%20%28double-precision%29))
  (Variables|Default|Sethealth (- (Variables|Default|Gethealth) damage))
  (if true
    _))