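; Interactable keypad actor that opens a referenced door when the player clicks in the correct code.
; Interacting blends the view to the keypad, frees the cursor and locks player movement and look; Q restores control.
; Clicked digit meshes feed Code, which updates the widget display and clears input after four digits.
; A match triggers the door's EnterInteract, turns the indicator green, shows a message and returns control.
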(event OnClicked(Keypad_button1)
  (params (TouchedComponent :type Primitive%20Component%20Object%20Reference) (ButtonPressed :type Key%20Structure :default "None"))
  (CallFunction|Code "1"))

(event OnClicked(Keypad_button2)
  (params (TouchedComponent :type Primitive%20Component%20Object%20Reference) (ButtonPressed :type Key%20Structure :default "None"))
  (CallFunction|Code "2"))

(event OnClicked(Keypad_button3)
  (params (TouchedComponent :type Primitive%20Component%20Object%20Reference) (ButtonPressed :type Key%20Structure :default "None"))
  (CallFunction|Code "3"))

(event OnClicked(Keypad_button4)
  (params (TouchedComponent :type Primitive%20Component%20Object%20Reference) (ButtonPressed :type Key%20Structure :default "None"))
  (CallFunction|Code "4"))

(event OnClicked(Keypad_button5)
  (params (TouchedComponent :type Primitive%20Component%20Object%20Reference) (ButtonPressed :type Key%20Structure :default "None"))
  (CallFunction|Code "5"))

(event OnClicked(Keypad_button6)
  (params (TouchedComponent :type Primitive%20Component%20Object%20Reference) (ButtonPressed :type Key%20Structure :default "None"))
  (CallFunction|Code "6"))

(event OnClicked(Keypad_button7)
  (params (TouchedComponent :type Primitive%20Component%20Object%20Reference) (ButtonPressed :type Key%20Structure :default "None"))
  (CallFunction|Code "7"))

(event OnClicked(Keypad_button8)
  (params (TouchedComponent :type Primitive%20Component%20Object%20Reference) (ButtonPressed :type Key%20Structure :default "None"))
  (CallFunction|Code "8"))

(event OnClicked(Keypad_button9)
  (params (TouchedComponent :type Primitive%20Component%20Object%20Reference) (ButtonPressed :type Key%20Structure :default "None"))
  (CallFunction|Code "9"))

(event OnClicked(Keypad_button0)
  (params (TouchedComponent :type Primitive%20Component%20Object%20Reference) (ButtonPressed :type Key%20Structure :default "None"))
  (CallFunction|Code "0"))

(event EventBeginPlay
  (bind _aswbp_keypad (Utilities|Casting|CastToWBP_Keypad (UserInterface|GetWidget (Variables|Default|GetWidget))))
  (Variables|Default|SetAs%20WBP%20Keypad _aswbp_keypad))

(event EventEnterInteract
  (bind _returnvalue (Game|GetPlayerController 0))
  (bind _returnvalue_2 (Game|GetPlayerController 0))
  (Game|Player|SetViewTargetwithBlend _returnvalue_2 self 0.3 "VTBlend_Linear" 0.0 false)
  (Input|SetIgnoreLookInput _returnvalue_2 true)
  (Variables|/Script/Engine.PlayerController|SetbEnableClickEvents _returnvalue_2 true)
  (Variables|/Script/Engine.PlayerController|SetbShowMouseCursor _returnvalue_2 true)
  (Pawn|Components|CharacterMovement|DisableMovement (Variables|/Script/Engine.Character|GetCharacterMovement (Game|GetPlayerCharacter 0)))
  (Input|EnableInput _returnvalue)
  (Input|SetInputModeGameandUI _returnvalue 0 "DoNotLock" true false))

(event Input|KeyboardEvents|Q
  (params (Key :type Key%20Structure :default "None"))
  (:Pressed
    (|Exit)))

(fn ConstructionScript)

(fn Code
  (params (B :type String))
  (bind _returnvalue (Game|GetPlayerController 0))
  (bind _returnvalue_2 (Game|GetPlayerCharacter 0))
  (Audio|PlaySound2D "/Game/KeyPad_Mechanic/Sound/key_code_sfx.key_code_sfx" 1.0 1.0 0.0 0 0)
  (bind _output_get (Variables|Default|SetInput (Utilities|String|Append (Variables|Default|GetInput) B)))
  (Variables|Default|SetCode_Length (+ (Variables|Default|GetCode_Length) 1))
  (Rendering|Components|TextRender|SetText (Variables|/Game/KeyPad_Mechanic/WBP_Keypad.WBP_Keypad_C|GetCode_Text (Variables|Default|GetAs%20WBP%20Keypad)) (Utilities|Text|ToText(String) _output_get))
  (if (Utilities|Enum|Equal(Enum) (Variables|Default|GetInput) (Variables|Default|GetCorrect_Code))
    (Class|BPIUnlockDoor|SetCodeCorrect(Message) (Game|GetPlayerCharacter 0) true)
    (Default|EnterInteract (Variables|Default|GetDoorREF))
    (Rendering|Material|SetMaterial (Variables|Default|GetKeypad_spheres) 0 "/Game/KeyPad_Mechanic/MI_KGreen.MI_KGreen")
    (Input|DisableInput _returnvalue)
    (Game|Player|SetViewTargetwithBlend _returnvalue _returnvalue_2 0.3 "VTBlend_Linear" 0.0 false)
    (Input|ResetIgnoreLookInput _returnvalue)
    (Variables|/Script/Engine.PlayerController|SetbEnableClickEvents _returnvalue false)
    (Variables|/Script/Engine.PlayerController|SetbShowMouseCursor _returnvalue false)
    (Pawn|Components|CharacterMovement|SetMovementMode (Variables|/Script/Engine.Character|GetCharacterMovement _returnvalue_2) "MOVE_Walking" 0)
    (Input|SetInputModeGameOnly _returnvalue false))
  (if (>= (Variables|Default|GetCode_Length) 4)
    (bind _output_get_2 (Variables|Default|SetInput ""))
    (Rendering|Components|TextRender|SetText (Variables|/Game/KeyPad_Mechanic/WBP_Keypad.WBP_Keypad_C|GetCode_Text (Variables|Default|GetAs%20WBP%20Keypad)) (Utilities|Text|ToText(String) _output_get_2))
    (Variables|Default|SetCode_Length 0)))